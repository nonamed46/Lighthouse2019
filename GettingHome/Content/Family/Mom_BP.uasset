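; Mom character Blueprint that shows a posed figure for a limited time, then removes it with a particle effect.
; On BeginPlay it holds a montage at zero play rate, attaches a paused Niagara system to the skeletal mesh, reveals a point light and starts a self-destruct timer.
; The Destroy event, apparently the timer's target, unpauses the particles and destroys the actor after a short delay.
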(event Custom|Destroy
  (Class|NiagaraComponent|SetPaused (Variables|Default|GetMeshEmitter_NIS) false)
  (Utilities|FlowControl|Delay 3.0)
  (Actor|DestroyActor))

(event EventBeginPlay
  (Animation|PlayAnimMontage (Variables|Default|GetMomAnimMontage) 0.0 "None")
  (bind _returnvalue (Niagara|SpawnSystemAttached "/Game/Effects/LightOutlines/NIS_MomMesh.NIS_MomMesh" (Variables|Default|GetSkeletalMesh) "None" "0, 0, 0" "0, 0, 0" "KeepRelativeOffset" false))
  (bind _output_get (Variables|Default|SetMeshEmitter_NIS _returnvalue))
  (Class|NiagaraComponent|SetPaused _output_get true)
  (Development|SetHiddeninGame (Variables|Default|GetPointLight) false false)
  (Utilities|Time|SetTimerbyEvent (EventDispatchers|CreateEvent :!event Custom|Destroy) (Variables|Default|GetSelfdestructTimer)))

(fn ConstructionScript)