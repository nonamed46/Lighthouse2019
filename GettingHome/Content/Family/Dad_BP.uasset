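; Dad apparition actor: a skeletal mesh frozen in its animation pose, paired with a mesh-based particle effect that later dissolves it.
; SpawnParticles attaches the NIS_DadMesh system to the mesh, pauses it almost immediately and reveals a point light.
; Destroy resumes the particles to dissolve, then removes the actor after a delay.
; PopulateVariables sets the scene and self-destruct timer, but the timer logic is disabled.
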(event Custom|Destroy
  ;[1 1 1] Lässt das PartikelSystem fortfahren (um sich aufzulösen) und Zerstört die Erscheinung.
  (Class|NiagaraComponent|SetPaused (Variables|Default|GetMeshEmitter_NIS) false)
  (Utilities|FlowControl|Delay 4.5)
  (Actor|DestroyActor))

(event Custom|SpawnParticles
  ;[1 1 1] Spawnt und Pausiert das angehängte Partikelsystem. Und macht ein Pointlight sichtbar.
  (bind _returnvalue (Niagara|SpawnSystemAttached "/Game/Effects/LightOutlines/NIS_DadMesh.NIS_DadMesh" (Variables|Default|GetSkeletalMesh) "None" "0, 0, 0" "0, 0, 0" "KeepRelativeOffset" false))
  (bind _output_get (Variables|Default|SetMeshEmitter_NIS _returnvalue))
  (Utilities|FlowControl|Delay 0.05)
  (Class|NiagaraComponent|SetPaused _output_get true)
  (Development|SetHiddeninGame (Variables|Default|GetPointLight) false false))

(event EventBeginPlay
  ;[1 1 1] Friert die Animationen ein.
  (Components|Timeline|SetPlayRate (Variables|Default|GetSkeletalMesh) 0.0))

(fn ConstructionScript)

(fn PopulateVariables
  (params (DadDestructionTimer :type Float%20%28single-precision%29) (currentScene :type Integer))
  (Variables|Default|SetSelfdestructTimer DadDestructionTimer)
  (Variables|Default|SetScene currentScene))