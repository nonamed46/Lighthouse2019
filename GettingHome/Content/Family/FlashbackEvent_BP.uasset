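; Flashback event actor that spawns and later removes Mom and Dad memory characters as the player walks through two trigger volumes.
; The spawn trigger fires once for the ThirdPersonCharacter, playing both parents' particle spawns and arming the destroy trigger, which destroys both and itself.
; The construction script passes the scene and self-destruct settings to both parents, though self-destruction is noted as currently inactive.
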(event OnComponentBeginOverlap(SpawnFlashback)
  (params (OverlappedComponent :type Primitive%20Component%20Object%20Reference) (OtherActor :type Actor%20Object%20Reference) (OtherComp :type Primitive%20Component%20Object%20Reference) (OtherBodyIndex :type Integer) (bFromSweep :type Boolean) (SweepResult :type Hit%20Result%20Structure%20%28by%20ref%29))
  (bind _dad (Variables|Default|GetDad))
  (bind _mom (Variables|Default|GetMom))
  (Utilities|Casting|CastToThirdPersonCharacter OtherActor)
  (Utilities|IsValid _dad
    (:Is%20Valid
      (Utilities|FlowControl|DoOnce false
        (:Completed
          (Variables|Default|SethasSpawned? true)
          (Default|SpawnParticles _dad)
          (Utilities|IsValid _mom
            (:Is%20Valid
              (Default|SpawnParticles _mom))))))
    (:Is%20Not%20Valid
      (Development|PrintString "Error: No Dad selected in FlashbackEvent"))))

(event OnComponentBeginOverlap(TriggerDestroyFlashback)
  (params (OverlappedComponent :type Primitive%20Component%20Object%20Reference) (OtherActor :type Actor%20Object%20Reference) (OtherComp :type Primitive%20Component%20Object%20Reference) (OtherBodyIndex :type Integer) (bFromSweep :type Boolean) (SweepResult :type Hit%20Result%20Structure%20%28by%20ref%29))
  (bind _dad (Variables|Default|GetDad))
  (bind _mom (Variables|Default|GetMom))
  (if (Variables|Default|GethasSpawned?)
    (Utilities|Casting|CastToThirdPersonCharacter OtherActor)
    (Utilities|IsValid _mom
      (:Is%20Valid
        (Utilities|FlowControl|DoOnce false
          (:Completed
            (Default|Destroy _mom)
            (Utilities|IsValid _dad
              (:Is%20Valid
                (Default|Destroy _dad))
              (:Is%20Not%20Valid
                _))
            (Actor|DestroyActor))))
      (:Is%20Not%20Valid
        (Development|PrintString "Error: No Mom selected in FlashbackEvent")))))

(fn ConstructionScript
  (bind _dad (Variables|Default|GetDad))
  (bind _mom (Variables|Default|GetMom))
  (bind _scene (Variables|Default|GetScene))
  ;[1 1 1] Befüllt die Charaktere mit den nötigen Infos. Selbstzerstörung ist derzeit inaktiv (müsste in Mom und Dad aktiviert werden)
  (Utilities|IsValid _dad
    (:Is%20Valid
      (Default|PopulateVariables _dad (Variables|Default|GetDadSelfdestruct) _scene)
      (Utilities|IsValid _mom
        (:Is%20Valid
          (Default|PopulateVariables _mom (Variables|Default|GetMomSelfdestruct) _scene))
        (:Is%20Not%20Valid
          (Development|PrintString "Error: No Mom selected in FlashbackEvent"))))
    (:Is%20Not%20Valid
      (Development|PrintString "Error: No Dad selected in FlashbackEvent"))))