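; WindsafeZone_BP is a trigger zone that changes the strength of wind, built from RadialForceActors, while the ThirdPersonCharacter is inside it.
; At BeginPlay it caches every RadialForceActor and stores force strength in one variable, keeping only the last actor's value.
; On begin overlap it sets all of their strengths to a fixed hardcoded value.
; On end overlap it applies that single stored strength to all of them.
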(event EventBeginPlay
  (bind _outactors (Actor|GetAllActorsOfClass "/Script/Engine.RadialForceActor"))
  (bind _output_get (Variables|Default|SetWindArray _outactors))
  (for _array_element _output_get
    (Variables|Default|SetInitialForce (Variables|/Script/Engine.RadialForceComponent|GetForceStrength (Variables|/Script/Engine.RadialForceActor|GetForceComponent _array_element)))))

(event Collision|EventActorBeginOverlap
  (params (OtherActor :type Actor%20Object%20Reference))
  (Utilities|Casting|CastToThirdPersonCharacter OtherActor)
  (for _array_element (Variables|Default|GetWindArray)
    (Variables|/Script/Engine.RadialForceComponent|SetForceStrength (Variables|/Script/Engine.RadialForceActor|GetForceComponent _array_element) 1e+05)))

(event Collision|EventActorEndOverlap
  (params (OtherActor :type Actor%20Object%20Reference))
  (Utilities|Casting|CastToThirdPersonCharacter OtherActor)
  (for _array_element (Variables|Default|GetWindArray)
    (Variables|/Script/Engine.RadialForceComponent|SetForceStrength (Variables|/Script/Engine.RadialForceActor|GetForceComponent _array_element) (Variables|Default|GetInitialForce))))

(fn ConstructionScript)