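; FogChange_BP is a trigger that thickens the level's height fog when the player character enters it.
; On BeginPlay it caches every ExponentialHeightFog actor in the level.
; When a ThirdPersonCharacter overlaps component R, it loops over that array and sets each fog component to a fixed, very high density.
; The file has no logic to restore the previous density.
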(event OnComponentBeginOverlap(r)
  (params (OverlappedComponent :type Primitive%20Component%20Object%20Reference) (OtherActor :type Actor%20Object%20Reference) (OtherComp :type Primitive%20Component%20Object%20Reference) (OtherBodyIndex :type Integer) (bFromSweep :type Boolean) (SweepResult :type Hit%20Result%20Structure%20%28by%20ref%29))
  (bind _fog (Variables|Default|GetFog))
  (Utilities|Casting|CastToThirdPersonCharacter OtherActor)
  (if (> (Utilities|Array|Length _fog) 0)
    (for _array_element _fog
      (Class|ExponentialHeightFogComponent|SetFogDensity (Variables|/Script/Engine.ExponentialHeightFog|GetComponent _array_element) 5e+01))))

(event EventBeginPlay
  (bind _outactors (Actor|GetAllActorsOfClass "/Script/Engine.ExponentialHeightFog"))
  (Variables|Default|SetFog _outactors))

(fn ConstructionScript)