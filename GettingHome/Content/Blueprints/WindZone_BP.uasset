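; A wind zone that switches the force components of its linked wind actors on and off while the ThirdPersonCharacter is inside.
; Entering starts with a calm phase via a DoOnce, and leaving shuts the wind off and resets it.
; WindBlow and WindOff toggle the forces, the character's IsInWindZone flag and audio fades.
; Each schedules a timer with its own duration, apparently to alternate gusts and lulls.
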(event Custom|WindBlow
  (bind _returnvalue (Game|GetPlayerCharacter 0))
  (if (Variables|Default|GetisBlowing)
    (bind _asthird_person_character (Utilities|Casting|CastToThirdPersonCharacter _returnvalue))
    (Variables|/Game/Player/ThirdPersonCharacter.ThirdPersonCharacter_C|SetIsInWindZone? _asthird_person_character true)
    (for _array_element (Variables|Default|GetWindArray)
      (bind _output_get (Variables|Default|SetWind _array_element))
      (Components|Activation|SetActive (Variables|/Script/Engine.RadialForceActor|GetForceComponent _output_get) true false)
      (Utilities|Time|SetTimerbyEvent (EventDispatchers|CreateEvent :!event Custom|WindOff) (Variables|Default|GetWindOn))
      (Audio|Components|Audio|FadeIn (Variables|Default|GetAudio) 0.5 1.0 0.0 :!class /Script/Engine.AudioComponent))
    (else
      (bind _asthird_person_character_2 (Utilities|Casting|CastToThirdPersonCharacter _returnvalue))
      (Variables|/Game/Player/ThirdPersonCharacter.ThirdPersonCharacter_C|SetIsInWindZone? _asthird_person_character_2 false)
      (for _array_element_2 (Variables|Default|GetWindArray)
        (bind _output_get_2 (Variables|Default|SetWind _array_element_2))
        (Components|Activation|SetActive (Variables|/Script/Engine.RadialForceActor|GetForceComponent _output_get_2) false false)
        (Audio|Components|Audio|FadeOut (Variables|Default|GetAudio) 0.5 0.0 :!class /Script/Engine.AudioComponent)))))

(event Custom|WindOff
  (bind _asthird_person_character (Utilities|Casting|CastToThirdPersonCharacter (Game|GetPlayerCharacter 0)))
  (Variables|/Game/Player/ThirdPersonCharacter.ThirdPersonCharacter_C|SetIsInWindZone? _asthird_person_character false)
  (for _array_element (Variables|Default|GetWindArray)
    (bind _output_get (Variables|Default|SetWind _array_element))
    (Components|Activation|SetActive (Variables|/Script/Engine.RadialForceActor|GetForceComponent _output_get) false false)
    (Audio|Components|Audio|FadeOut (Variables|Default|GetAudio) 0.5 0.0 :!class /Script/Engine.AudioComponent)
    (Utilities|Time|SetTimerbyEvent (EventDispatchers|CreateEvent :!event Custom|WindBlow) (Variables|Default|GetWindNotOn))))

(event Collision|EventActorBeginOverlap
  (params (OtherActor :type Actor%20Object%20Reference))
  (Utilities|Casting|CastToThirdPersonCharacter OtherActor)
  (Variables|Default|SetisBlowing true)
  (Utilities|FlowControl|DoOnce false
    (:Completed
      (CallFunction|WindOff))))

(event Collision|EventActorEndOverlap
  (params (OtherActor :type Actor%20Object%20Reference))
  (Utilities|Casting|CastToThirdPersonCharacter OtherActor)
  (Variables|Default|SetisBlowing false)
  (CallFunction|WindBlow)
  (Utilities|FlowControl|DoOnce false) ; enters at Reset
)

(fn ConstructionScript)