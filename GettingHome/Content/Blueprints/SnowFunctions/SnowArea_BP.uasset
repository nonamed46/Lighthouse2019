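; SnowArea_BP is an actor that follows the player pawn and publishes its snow area's placement to materials.
; Each tick it writes its up vector and the Snow component's world location to the MPC_SnowDepth material parameter collection, then moves itself to player pawn 0's location.
; The construction script runs the same update, so the collection is also set when the actor is constructed.
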(event Custom|UpdateLocation
  (Rendering|Material|SetVectorParameterValue "/Game/Blueprints/SnowFunctions/MPC_SnowDepth.MPC_SnowDepth" "UpVector" (Math|Conversions|ToLinearColor(Vector) (Transformation|GetActorUpVector)) :!class /Script/Engine.KismetMaterialLibrary)
  (Rendering|Material|SetVectorParameterValue "/Game/Blueprints/SnowFunctions/MPC_SnowDepth.MPC_SnowDepth" "ParticleLocation" (Math|Conversions|ToLinearColor(Vector) (Transformation|GetWorldLocation (Variables|Default|GetSnow))) :!class /Script/Engine.KismetMaterialLibrary))

(event EventTick
  (params (DeltaSeconds :type Float%20%28single-precision%29))
  (CallFunction|UpdateLocation)
  (Transformation|SetActorLocation (Transformation|GetActorLocation (Game|Player|GetPlayerPawn 0)) false false))

(fn ConstructionScript
  (CallFunction|UpdateLocation))