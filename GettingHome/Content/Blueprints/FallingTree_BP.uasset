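; FallingTree_BP is an interactable tree that falls over once when the Interact event fires.
; BeginPlay caches the Tree component's initial roll and yaw.
; Interact passes a DoOnce gate, plays the Baumstumpf sound at the actor's location and starts the Falling timeline.
; The timeline's FallingZRot track drives the relative pitch of TreePivot, with the cached roll and yaw applied alongside.
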(event EventInteract
  (Utilities|FlowControl|DoOnce false
    (:Completed
      (Audio|PlaySoundatLocation "/Game/Audio/Baumstumpf.Baumstumpf" (Transformation|GetActorLocation self) "0, 0, 0" 1.0 1.0 0.0 0 0 0)
      (bind _fallingzrot (Timeline|Falling Play)
        (:Update
          (Transformation|SetRelativeRotation (Variables|Default|GetTreePivot) (Math|Rotator|MakeRotator (stale EventBeginPlay _output_get) _fallingzrot (stale EventBeginPlay _output_get_2)) false false))))))

(event EventBeginPlay
  (bind _tree (Variables|Default|GetTree))
  (bind _relativerotation (Variables|/Script/Engine.SceneComponent|GetRelativeRotation _tree))
  (bind _output_get (Variables|Default|SettreeOriginXRot (.roll _relativerotation)))
  (bind _output_get_2 (Variables|Default|SettreeOriginZRot (.yaw _relativerotation))))

(fn ConstructionScript)