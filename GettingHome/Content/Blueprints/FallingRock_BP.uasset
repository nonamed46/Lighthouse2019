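; FallingRock_BP is a rock hazard that falls when the third-person character enters its trigger box.
; The first overlap enables physics on the mesh, applies a sideways and downward impulse, plays a rockfall sound and destroys the trigger.
; A timer then repeatedly polls the mesh's velocity and switches physics simulation off once the rock comes to rest.
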(event OnComponentBeginOverlap(TriggerBox)
  (params (OverlappedComponent :type Primitive%20Component%20Object%20Reference) (OtherActor :type Actor%20Object%20Reference) (OtherComp :type Primitive%20Component%20Object%20Reference) (OtherBodyIndex :type Integer) (bFromSweep :type Boolean) (SweepResult :type Hit%20Result%20Structure%20%28by%20ref%29))
  (bind _staticmesh (Variables|Default|GetStaticMesh))
  (Utilities|Casting|CastToThirdPersonCharacter OtherActor)
  (Utilities|FlowControl|DoOnce false
    (:Completed
      (Physics|SetSimulatePhysics _staticmesh true)
      (Physics|AddImpulse _staticmesh "0,200.000000,-500.000000" "None" false)
      (Audio|PlaySoundatLocation "/Game/Audio/GrosserSteinschlag.GrosserSteinschlag" (Transformation|GetActorLocation) "0, 0, 0" 1.0 1.0 0.0 0 0 0)
      (Utilities|Time|SetTimerbyEvent (delegate Custom|CheckVelocity) 2.0)
      (Components|DestroyComponent (Variables|Default|GetTriggerBox)))))

(event Custom|CheckVelocity
  (bind _returnvalue (Physics|GetPhysicsLinearVelocity (Variables|Default|GetStaticMesh) "None"))
  (if (<= (Math|Vector|VectorLength _returnvalue) 0.1)
    (Physics|SetSimulatePhysics (Variables|Default|GetStaticMesh) false)
    (Development|PrintString "physics off")
    (else
      (Utilities|Time|SetTimerbyEvent (delegate Custom|CheckVelocity) 0.5))))

(fn ConstructionScript)